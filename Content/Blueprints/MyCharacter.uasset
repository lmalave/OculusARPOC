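; MyCharacter is a character Blueprint that maps keyboard and mouse wheel input to controls for in-world web browser windows.
; Number keys 1–3 spawn windows along the camera direction, each with a hardcoded URL, scale, pixel width and distance.
; Tab toggles window move mode, the wheel zooms windows in and out, and M calls SpawnAtMarker.
; The graph only forwards input, with the window logic defined outside it.
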(event `Key|One`
  (:`Pressed`
    (`self.SpawnUIWindowAtCameraDirectionWithParams` "http://www.hugeinc.com" 1.0 0.7 1200.0 100.0)))

(event `Key|MouseScrollDown`
  (:`Pressed`
    (`self.HandleZoomOutWindow`)))

(event `Key|Tab`
  (:`Pressed`
    (`self.ToggleWindowMoveMode`)))

(event `Key|MouseScrollUp`
  (:`Pressed`
    (`self.HandleZoomInWindow`)))

(event `Key|M`
  (:`Pressed`
    (`self.SpawnAtMarker`)))

(event `Key|Three`
  (:`Pressed`
    (`self.SpawnUIWindowAtCameraDirectionWithParams` "http://weather.com" 0.35 0.35 600.0 100.0)))

(event `Key|Two`
  (:`Pressed`
    (`self.SpawnUIWindowAtCameraDirectionWithParams` "http://www.bloomberg.com/markets/world/" 0.35 0.45 600.0 50.0)))

(fn `UserConstructionScript`)